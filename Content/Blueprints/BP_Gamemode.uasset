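; BP_Gamemode is a game mode that shows a live on-screen debug readout of a GOAP AI controller.
; On Tick, it finds and caches a BP_GOAPAIController whenever the stored reference is invalid.
; While the reference is valid, it prints that controller's State map and GoalState map under colored headings, using keyed PrintString calls so lines update in place.
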(event EventBeginPlay)

(event EventTick
  (params (DeltaSeconds :type Float%20%28single-precision%29))
  (Utilities|IsValid (Variables|Default|GetRandomGOAPController)
    (:Is%20Valid
      (Development|PrintString "Controller 1:" true true "(R=1.000000,G=0.093725,B=0.000348,A=1.000000)" 2.0 "Title")
      (bind (_keypin _valuepin) (Utilities|Map|ForEachLoop(Map) (Variables|/Script/AIResearch.GOAPAIController|GetState (Variables|Default|GetRandomGOAPController)))
        (:then
          (Development|PrintString (Utilities|String|Append (Utilities|String|ToString(Name) _keypin) " :" (Utilities|String|ToString(Boolean) _valuepin)) true true "(R=0.000000,G=0.660000,B=1.000000,A=1.000000)" 2.0 _keypin))
        (:CompletedPin
          (Development|PrintString "GOAL:" true true "(R=1.000000,G=0.093725,B=0.000348,A=1.000000)" 2.0 "Title2")
          (bind (_keypin_2 _valuepin_2) (Utilities|Map|ForEachLoop(Map) (Variables|/Script/AIResearch.GOAPAIController|GetGoalState (Variables|Default|GetRandomGOAPController)))
            (:then
              (Development|PrintString (Utilities|String|Append (Utilities|String|ToString(Name) _keypin_2) " :" (Utilities|String|ToString(Boolean) _valuepin_2)) true true "(R=0.000000,G=0.660000,B=1.000000,A=1.000000)" 2.0 (Utilities|String|StringToName (Utilities|String|Append (Utilities|String|ToString(Name) _keypin_2) "2"))))))))
    (:Is%20Not%20Valid
      (bind _returnvalue (Actor|GetActorOfClass "/Game/Blueprints/BP_GOAPAIController.BP_GOAPAIController_C"))
      (Variables|Default|SetRandomGOAPController _returnvalue))))

(fn ConstructionScript)